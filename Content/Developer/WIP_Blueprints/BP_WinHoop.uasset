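; BP_WinHoop is a work-in-progress basketball hoop that checks whether a BP_ThrowableBasketball passes two trigger spheres in the correct order.
; Overlapping Sphere arms a point flag, which clears after a short delay once the ball leaves it.
; Overlapping Sphere1 while armed calls PointTally and disarms; otherwise it prints "Cheater".
; PointTally is an empty stub, and the point-gained message is unconnected.
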(event `self.Sphere.OnComponentBeginOverlap`
  (params (OverlappedComponent :type "PrimitiveComponent Object Reference") (OtherActor :type "Actor Object Reference") (OtherComp :type "PrimitiveComponent Object Reference") (OtherBodyIndex :type Integer) (bFromSweep :type Boolean) (SweepResult :type "HitResult Structure (by ref)"))
  (cast `/Game/StealthGame/Gadgets/NoiseMakers/BP_ThrowableBasketball` OtherActor)
  (set `self.bHitSphere0` true)
  (if (`self.bHitSphere0`)
    (set `self.bPointConditionSet` true)
    (else
      (`KismetSystemLibrary.PrintString` "Cheater"))))

(event `PointTally`)

(event `self.Sphere.OnComponentEndOverlap`
  (params (OverlappedComponent :type "PrimitiveComponent Object Reference") (OtherActor :type "Actor Object Reference") (OtherComp :type "PrimitiveComponent Object Reference") (OtherBodyIndex :type Integer))
  (cast `/Game/StealthGame/Gadgets/NoiseMakers/BP_ThrowableBasketball` OtherActor)
  (`KismetSystemLibrary.Delay` 3.0)
  (set `self.bPointConditionSet` false))

(event `self.Sphere1.OnComponentBeginOverlap`
  (params (OverlappedComponent :type "PrimitiveComponent Object Reference") (OtherActor :type "Actor Object Reference") (OtherComp :type "PrimitiveComponent Object Reference") (OtherBodyIndex :type Integer) (bFromSweep :type Boolean) (SweepResult :type "HitResult Structure (by ref)"))
  (cast `/Game/StealthGame/Gadgets/NoiseMakers/BP_ThrowableBasketball` OtherActor)
  (if (`self.bPointConditionSet`)
    (`self.PointTally`)
    (set `self.bPointConditionSet` false)
    (else
      (`KismetSystemLibrary.PrintString` "Cheater"))))

(fn `UserConstructionScript`)